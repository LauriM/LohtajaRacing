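; Kaljaa is a beer pickup that the game's vehicle collects, and it counts toward victory.
; An overlap on its collision sphere plays the beer-opening sound at its location and destroys the actor.
; It then increments the current and total beer counters on every VehicleBlueprint in the level, setting that vehicle's victory flag once its total passes a hardcoded threshold.
; The overlapping actor is never checked, so any overlap triggers collection.
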(event `self.CollisionSprehe.OnComponentBeginOverlap`
  (params (OtherActor :type "Actor Object Reference") (OtherComp :type "PrimitiveComponent Object Reference") (OtherBodyIndex :type Integer) (bFromSweep :type Boolean) (SweepResult :type "EngineTypes.HitResult Structure (by ref)"))
  (`GameplayStatics.PlaySoundAtLocation` "/Game/Sound/Beeropen.Beeropen" (`self.K2_GetActorLocation`))
  (`self.K2_DestroyActor`)
  (bind _outactors (`GameplayStatics.GetAllActorsOfClass` "/Game/Vehicle/VehicleBlueprint.VehicleBlueprint_C"))
  (for _array_element _outactors
    (set `/Game/Vehicle/VehicleBlueprint.kalja_Amount` (+ (`/Game/Vehicle/VehicleBlueprint.kalja_Amount` _array_element) 1) _array_element)
    ;[1 1 1] victory counter
    (set `/Game/Vehicle/VehicleBlueprint.total_kalja_count` (+ (`/Game/Vehicle/VehicleBlueprint.total_kalja_count` _array_element) 1) _array_element)
    ;[1 1 1] victory check
    (if (> (`/Game/Vehicle/VehicleBlueprint.total_kalja_count` _array_element) 28)
      (set `/Game/Vehicle/VehicleBlueprint.VICTORY_HAS_BEEN_ACHIEVED` true _array_element))))

(fn `UserConstructionScript`)