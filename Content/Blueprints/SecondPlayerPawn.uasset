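; Second player pawn, apparently a spectator camera, that follows a VehicleBlueprint actor in the level.
; The construction script moves it to a fixed debug location, then loops over all vehicles, storing and attaching to each, so the last one wins.
; Each Tick snaps it to player controller 0's transform, then immediately overrides that with the vehicle's transform.
; Debug prints trace setup and every tick.
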(event `self.ReceiveTick`
  (params (DeltaSeconds :type "Float (single-precision)"))
  (`KismetSystemLibrary.PrintString` "tick")
  (`|ExecutionSequence`
    (:`then_0`
      (`self.K2_SetActorTransform` (`self.GetTransform` (`GameplayStatics.GetPlayerController` 0))))
    (:`then_1`
      (`self.K2_SetActorTransform` (`self.GetTransform` (`self.Vehicle`))))))

(fn `UserConstructionScript`
  ;[1 1 1] Debug testing
  (`self.K2_SetActorLocation` (-7000.0 9000.0 200.0))
  (`KismetSystemLibrary.PrintString` "SPECTATOR CAMERA UP")
  (bind _outactors (`GameplayStatics.GetAllActorsOfClass` "/Game/Vehicle/VehicleBlueprint.VehicleBlueprint_C"))
  (for _array_element _outactors
    (set `self.Vehicle` _array_element)
    (`KismetSystemLibrary.PrintString` "VEHICLE FOUND")
    (`self.K2_AttachRootComponentToActor` (`self.Vehicle`))
    (`KismetSystemLibrary.PrintString` "Actor to Actor attach done!")))